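; BP_StellarGM, apparently the Stellar game mode, applies saved audio settings and starts looping background music on BeginPlay.
; It loads the "sound" save slot as SG_Sound, first creating and saving a default one if none exists.
; The saved Master, Music and SFX volumes feed class overrides on StellarSoundMix, then MusicLoop fades in as a 2D sound.
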(event `self.ReceiveBeginPlay`
  (`|ExecutionSequence`
    (:`then_0`
      (bind _returnvalue (`GameplayStatics.DoesSaveGameExist` "sound"))
      (if (not _returnvalue)
        (bind _returnvalue_2 (`GameplayStatics.CreateSaveGameObject` "/Game/Blueprints/Misc/SG_Sound.SG_Sound_C"))
        (`GameplayStatics.SaveGameToSlot` _returnvalue_2 "sound"))
      (bind _returnvalue_3 (`GameplayStatics.LoadGameFromSlot` "sound"))
      (bind _assg_sound (cast `/Game/Blueprints/Misc/SG_Sound` _returnvalue_3))
      (`GameplayStatics.SetSoundMixClassOverride` "/Game/Blueprints/Misc/StellarSoundMix.StellarSoundMix" "/Engine/EngineSounds/Master.Master" (`/Game/Blueprints/Misc/SG_Sound.MasterVolume` _assg_sound) 1.0 0.0)
      (`GameplayStatics.SetSoundMixClassOverride` "/Game/Blueprints/Misc/StellarSoundMix.StellarSoundMix" "/Engine/EngineSounds/Music.Music" (`/Game/Blueprints/Misc/SG_Sound.MusicVolume` _assg_sound))
      (`GameplayStatics.SetSoundMixClassOverride` "/Game/Blueprints/Misc/StellarSoundMix.StellarSoundMix" "/Engine/EngineSounds/SFX.SFX" (`/Game/Blueprints/Misc/SG_Sound.SFXVolume` _assg_sound)))
    (:`then_1`
      (bind _returnvalue_4 (`GameplayStatics.CreateSound2D` "/Game/Sounds/MusicLoop.MusicLoop" 1.0 1.0 0.0 null))
      (`AudioComponent.FadeIn` _returnvalue_4 1.0 1.0 0.0 "Linear"))))

(fn `UserConstructionScript`)