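; Blueprint function library of trace helpers that probe a cone of directions around an actor's forward vector.
; The cone functions tilt the forward vector by the cone angle, spin it evenly around that axis, and map each location to its blocking-hit flag.
; The line variant stores trace ends; the capsule-sized sphere variant stores hit locations when blocked and ignores the player.
; A third helper returns the point straight ahead at trace length.
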(fn CreateConeTraceLocations
  (params (TraceAmount :type Integer) (Actor :type Actor%20Object%20Reference) (TraceLength :type Float%20%28double-precision%29) (ConeAngle :type Float%20%28double-precision%29))
  (bind _returnvalue (Transformation|GetActorLocation Actor))
  (Utilities|Map|Clear (LocalVariables|GetLocations))
  (for _index (range 0 (- TraceAmount 1))
    (bind _outhit (Collision|LineTraceByChannel 0 _returnvalue (|((V*TL)+Loc) (Math|Vector|RotateVectorAroundAxis (Math|Vector|RotateVectorAroundAxis (Transformation|GetActorForwardVector Actor) ConeAngle (Transformation|GetActorRightVector Actor)) (|((X/TraceA)*I) 3.6e+02 TraceAmount _index) (Transformation|GetActorForwardVector Actor)) TraceLength _returnvalue) "TraceTypeQuery1" false (Utilities|Array|MakeArray Actor) "ForOneFrame"))
    (Utilities|Map|Add (LocalVariables|GetLocations) (.TraceEnd (Collision|BreakHitResult _outhit)) (.bBlockingHit (Collision|BreakHitResult _outhit))))
  (return (LocalVariables|GetLocations)))

(fn TraceForwardEndPoint
  (params (Actor :type Actor%20Object%20Reference) (TraceLength :type Float%20%28double-precision%29))
  (return (+ (* (Transformation|GetActorForwardVector Actor) TraceLength) (Transformation|GetActorLocation Actor))))

(fn CreateConeSphereTraceLocations
  (params (TraceAmount :type Integer) (Actor :type Actor%20Object%20Reference) (TraceLength :type Float%20%28double-precision%29) (ConeAngle :type Float%20%28double-precision%29))
  (bind _returnvalue (Transformation|GetActorLocation Actor))
  (Utilities|Map|Clear (LocalVariables|GetNonHitLocations))
  (for _index (range 0 (- TraceAmount 1))
    (bind _outhit (Collision|SphereTraceByChannel Actor _returnvalue (+ (* (Math|Vector|RotateVectorAroundAxis (Math|Vector|RotateVectorAroundAxis (Transformation|GetActorForwardVector Actor) ConeAngle (Transformation|GetActorRightVector Actor)) (|((X/TraceA)*I) 3.6e+02 TraceAmount _index) (Transformation|GetActorForwardVector Actor)) TraceLength) _returnvalue) (+ (Variables|/Script/Engine.CapsuleComponent|GetCapsuleRadius (Actor|GetComponentbyClass Actor "/Script/Engine.CapsuleComponent")) 1e+01) "TraceTypeQuery1" false (Utilities|Array|MakeArray Actor (Game|GetPlayerCharacter Actor)) "None"))
    (if (.bBlockingHit (Collision|BreakHitResult _outhit))
      (Utilities|Map|Add (LocalVariables|GetNonHitLocations) (.Location (Collision|BreakHitResult _outhit)) (.bBlockingHit (Collision|BreakHitResult _outhit)))
      (else
        (Utilities|Map|Add (LocalVariables|GetNonHitLocations) (.TraceEnd (Collision|BreakHitResult _outhit)) (.bBlockingHit (Collision|BreakHitResult _outhit))))))
  (return (LocalVariables|GetNonHitLocations)))