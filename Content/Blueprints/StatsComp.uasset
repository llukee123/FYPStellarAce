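; Stats component that tracks a current health value against a maximum and signals death.
; UpdateHealth adds a signed change to CurrentHealth, clamps the result between zero and MaxHealth, then calls Death when health is at or below zero.
; An initial below-zero check has both branches empty, so the clamp alone bounds the value.
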(fn `UpdateHealth`
  (params (HealthChange :type "Float (double-precision)"))
  (bind _returnvalue (+ HealthChange (`self.CurrentHealth`)))
  (if (< _returnvalue 0.0)
    _
    (else
      _))
  (bind _output_get (set `self.CurrentHealth` (`KismetMathLibrary.FClamp` _returnvalue 0.0 (`self.MaxHealth`))))
  (if (<= _output_get 0.0)
    (`self.Death`))
  (return))