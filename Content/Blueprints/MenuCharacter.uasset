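; MenuCharacter is a menu character that lets Enhanced Input actions drive the mouse cursor and send clicks.
; On BeginPlay it adds the default mapping context to player controller 0.
; The look action nudges the OS mouse position by its scaled axis values, acting as a virtual cursor.
; The shoot action sends a left mouse button key press and release through a WidgetInteraction component.
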(event `self.ReceiveBeginPlay`
  (bind _returnvalue (pcsubsystem `EnhancedInputLocalPlayerSubsystem` (`GameplayStatics.GetPlayerController` 0)))
  (`/Engine/EditorBlueprintResources/StandardMacros.IsValid` _returnvalue
    (:`Is Valid`
      (`EnhancedInputSubsystemInterface.AddMappingContext` _returnvalue "/Game/Input/IMC_Default.IMC_Default" 0 (struct)))))

(event `EnhancedInput|/Game/Input/Actions/IA_Look1`
  (params (ActionValue :type "Vector2D Structure") (ElapsedSeconds :type "Float (double-precision)") (TriggeredSeconds :type "Float (double-precision)") (InputAction :type "InputAction Object Reference" :default "/Game/Input/Actions/IA_Look1.IA_Look1"))
  (bind (_locationx _locationy) (`PlayerController.GetMousePosition` (`GameplayStatics.GetPlayerController` 0)))
  (:`Triggered`
    (`PlayerController.SetMouseLocation` (`GameplayStatics.GetPlayerController` 0) (`KismetMathLibrary.Round` (+ _locationx (* ActionValue_X 20.0))) (`KismetMathLibrary.Round` (+ _locationy (* ActionValue_Y 20.0))))))

(event `EnhancedInput|/Game/Input/Actions/IA_Shoot1`
  (params (ActionValue :type Boolean) (ElapsedSeconds :type "Float (double-precision)") (TriggeredSeconds :type "Float (double-precision)") (InputAction :type "InputAction Object Reference" :default "/Game/Input/Actions/IA_Shoot1.IA_Shoot1"))
  (:`Started`
    (`WidgetInteractionComponent.PressAndReleaseKey` (`self.WidgetInteraction`) "LeftMouseButton")))

(fn `UserConstructionScript`)